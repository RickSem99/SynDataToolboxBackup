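; Actor component implementing a PID controller, with a Reset that clears the stored integral and previous error.
; PID takes target, current value and limits, weights proportional, integral and derivative terms by the Gains vector, and clamps the output.
; As shown, the computed Error is unused: the terms and stored error take zero in its place.
; An optional Debug flag prints integral, error and output on screen.
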(fn `PID`
  (params (Target :type "Float (double-precision)") (Current :type "Float (double-precision)") (Min :type "Float (double-precision)") (Max :type "Float (double-precision)"))
  (returns (Output :type "Float (double-precision)"))
  (locals (Error :type "Float (double-precision)") (Integral :type "Float (double-precision)") (Derived :type "Float (double-precision)"))
  (bind (_gains_x _gains_y _gains_z) (`KismetMathLibrary.BreakVector` (`self.Gains`)))
  (set `local.Error` (- (`local.Target`) (`local.Current`)))
  (set `local.Integral` (+ (* 0.0 (`GameplayStatics.GetWorldDeltaSeconds`)) (`self.LastIntegral`)))
  (set `local.Derived` (/ (- 0.0 (`self.LastError`)) (`GameplayStatics.GetWorldDeltaSeconds`)))
  (set `self.Output` (`KismetMathLibrary.FClamp` (+ (* _gains_x 0.0) (* _gains_y (`local.Integral`)) (* _gains_z (`local.Derived`))) (`local.Min`) (`local.Max`)))
  (set `self.LastIntegral` (`local.Integral`))
  (set `self.LastError` 0.0)
  (if (`self.Debug`)
    (`KismetSystemLibrary.PrintString` (`KismetTextLibrary.Conv_TextToString` (`|FormatText` "I:{i} E:{e} O:{o}" (`KismetTextLibrary.Conv_DoubleToText` (`local.Integral`) "HalfToEven" false true 1 324 2 2) (`KismetTextLibrary.Conv_DoubleToText` 0.0 "HalfToEven" false true 1 324 2 2) (`KismetTextLibrary.Conv_DoubleToText` (`self.Output`) "HalfToEven" false true 1 324 2 2))) true false (`self.Debug Color`) 0.0))
  (return (`self.Output`)))

(fn `Reset`
  (set `self.LastIntegral` 0.0)
  (set `self.LastError` 0.0))