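; BP_Volume is a utility actor that exports the world-space bounds of its BoxVolume reference to a text file.
; On BeginPlay it reads the volume's origin and box extent, derives the min and max of each axis, and joins them into one labelled string.
; It writes that string to VolumeMisure.txt in the project's Saved directory, printing an on-screen confirmation when the save succeeds.
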(event `self.ReceiveBeginPlay`
  (bind (_origin _boxextent) (`self.GetActorBounds` (`self.BoxVolume`) false false))
  (bind _x (.x _boxextent))
  (bind _y (.y _boxextent))
  (bind _z (.z _boxextent))
  (bind _x_2 (.x _origin))
  (bind _y_2 (.y _origin))
  (bind _z_2 (.z _origin))
  (bind _returnvalue (`AdvancedSaveSystemBPLibrary.SaveStringToFile` (`KismetStringLibrary.Concat_StrStr` "MinX:" (`KismetStringLibrary.Conv_DoubleToString` (- _x_2 _x)) " \nMaxX: " (`KismetStringLibrary.Conv_DoubleToString` (+ _x_2 _x)) " \nMinY: " (`KismetStringLibrary.Conv_DoubleToString` (- _y_2 _y)) " \nMaxY: " (`KismetStringLibrary.Conv_DoubleToString` (+ _y_2 _y)) " \nMinZ: " (`KismetStringLibrary.Conv_DoubleToString` (- _z_2 _z)) " \nMaxZ: " (`KismetStringLibrary.Conv_DoubleToString` (+ _z_2 _z))) (`KismetSystemLibrary.GetProjectSavedDirectory`) "VolumeMisure" ".txt"))
  (`KismetSystemLibrary.PrintString` "File salvato correttamente" _returnvalue))

(fn `UserConstructionScript`)